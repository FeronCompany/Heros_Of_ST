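; BP_MainView is a player-controlled camera view that pans and zooms using input actions and mouse edge scrolling.
; IA_Move shifts the actor along world X and Y, while IA_Zoom changes SpringArm length only when the result stays within fixed bounds.
; Each Tick, ViewPortCheck detects the cursor in the viewport's edge margins and offsets the actor along its forward and right vectors.
; ControlSensitivity scales all three controls.
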(event Input|EnhancedActionEvents|EnhancedInputActionIA_Move
  (params (ActionValue :type Vector%202D%20Structure) (ElapsedSeconds :type Float%20%28double-precision%29) (TriggeredSeconds :type Float%20%28double-precision%29) (InputAction :type Input%20Action%20Object%20Reference :default "/Game/controller/IA_Move.IA_Move"))
  (bind _returnvalue (Transformation|GetActorLocation))
  (bind _control_sensitivity (Variables|Default|Getcontrol_sensitivity))
  (Transformation|SetActorLocation (Math|Vector|MakeVector (+ (* (.x ActionValue) _control_sensitivity) (.x _returnvalue)) (+ (* (.y ActionValue) _control_sensitivity) (.y _returnvalue)) (.z _returnvalue)) false false))

(event Input|EnhancedActionEvents|EnhancedInputActionIA_Zoom
  (params (ActionValue :type Float%20%28double-precision%29) (ElapsedSeconds :type Float%20%28double-precision%29) (TriggeredSeconds :type Float%20%28double-precision%29) (InputAction :type Input%20Action%20Object%20Reference :default "/Game/controller/IA_Zoom.IA_Zoom"))
  (bind _springarm (Variables|Default|GetSpringArm))
  (if (and (> (+ (* ActionValue (Variables|Default|Getcontrol_sensitivity) 3.0) (Variables|/Script/Engine.SpringArmComponent|GetTargetArmLength _springarm)) -3e+02) (< (+ (* ActionValue (Variables|Default|Getcontrol_sensitivity) 3.0) (Variables|/Script/Engine.SpringArmComponent|GetTargetArmLength _springarm)) 2e+02))
    (Variables|/Script/Engine.SpringArmComponent|SetTargetArmLength _springarm (+ (* ActionValue (Variables|Default|Getcontrol_sensitivity) 3.0) (Variables|/Script/Engine.SpringArmComponent|GetTargetArmLength _springarm)))))

(event EventBeginPlay)

(event Collision|EventActorBeginOverlap
  (params (OtherActor :type Actor%20Object%20Reference)))

(event EventTick
  (params (DeltaSeconds :type Float%20%28single-precision%29))
  (CallFunction|ViewPortCheck DeltaSeconds))

(fn ConstructionScript)

(fn ViewPortCheck
  (params (deltaTime :type Float%20%28double-precision%29))
  (bind _returnvalue (Viewport|GetViewportSize))
  (bind _returnvalue_2 (Transformation|GetActorRightVector))
  (bind _returnvalue_3 (Transformation|GetActorForwardVector))
  (bind _as玩家控制器 (Utilities|Casting|CastToPlayerController (Pawn|GetController)))
  (if (and (<= (.LocationX (Game|Player|GetMousePosition _as玩家控制器)) (* (.x _returnvalue) 0.05)) (> (.LocationX (Game|Player|GetMousePosition _as玩家控制器)) 0.0))
    (LocalVariables|SetdeltaMovement (- (LocalVariables|GetdeltaMovement) _returnvalue_2))
    (elif (and (>= (.LocationX (Game|Player|GetMousePosition _as玩家控制器)) (* (.x _returnvalue) 0.95)) (<= (.LocationX (Game|Player|GetMousePosition _as玩家控制器)) (.x _returnvalue)))
      (LocalVariables|SetdeltaMovement (+ _returnvalue_2 (LocalVariables|GetdeltaMovement)))))
  (if (and (<= (.LocationY (Game|Player|GetMousePosition _as玩家控制器)) (* (.y _returnvalue) 0.05)) (> (.LocationY (Game|Player|GetMousePosition _as玩家控制器)) 0.0))
    (LocalVariables|SetdeltaMovement (+ (LocalVariables|GetdeltaMovement) _returnvalue_3))
    (elif (and (>= (.LocationY (Game|Player|GetMousePosition _as玩家控制器)) (* (.y _returnvalue) 0.95)) (<= (.LocationY (Game|Player|GetMousePosition _as玩家控制器)) (.y _returnvalue)))
      (LocalVariables|SetdeltaMovement (- (LocalVariables|GetdeltaMovement) _returnvalue_3))))
  (Transformation|AddActorWorldOffset (* (LocalVariables|GetdeltaMovement) (* 1e+02 (Variables|Default|Getcontrol_sensitivity) deltaTime))))
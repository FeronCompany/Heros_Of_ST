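; Main player controller that handles cursor-based actor highlighting and picking, the HUD widgets, and pausing.
; Each tick a visibility trace under the cursor highlights actors implementing BI_CursorDetector and tracks the last one hit.
; Pick input toggles or switches selection of that hovered actor through interface messages, hiding character info on empty clicks.
; It creates main, character info and pause menu widgets, swapping their visibility when pause input toggles the game.
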(event Input|EnhancedActionEvents|EnhancedInputActionIA_PickItem
  (params (ActionValue :type Boolean) (ElapsedSeconds :type Float%20%28double-precision%29) (TriggeredSeconds :type Float%20%28double-precision%29) (InputAction :type Input%20Action%20Object%20Reference :default "/Game/controller/IA_PickItem.IA_PickItem"))
  (:Completed
    (CallFunction|PickCheck)))

(event Input|EnhancedActionEvents|EnhancedInputActionIA_Pause
  (params (ActionValue :type Boolean) (ElapsedSeconds :type Float%20%28double-precision%29) (TriggeredSeconds :type Float%20%28double-precision%29) (InputAction :type Input%20Action%20Object%20Reference :default "/Game/controller/IA_Pause.IA_Pause"))
  (:Completed
    (if (Variables|Default|GetIsPaused)
      (CallFunction|ResumeGame)
      (else
        (CallFunction|PauseGame)))))

(event EventBeginPlay
  (Input|AddMappingContext (PlayerController|LocalPlayerSubsystems|GetEnhancedInputLocalPlayerSubsystem) "/Game/controller/IMC_MainCamera.IMC_MainCamera" 0 "(bIgnoreAllPressedKeysUntilRelease=True,bForceImmediately=False,bNotifyUserSettings=False)")
  (Variables|Default|SetbShowMouseCursor true)
  (CallFunction|InitUI)
  (Input|SetInputModeGameandUI self 0 "DoNotLock" false false))

(event EventTick
  (params (DeltaSeconds :type Float%20%28single-precision%29))
  (CallFunction|CursorTrace))

(fn ConstructionScript)

(fn CursorTrace
  (bind (_hitresult _returnvalue) (Game|Player|GetHitResultUnderCursorbyChannel "TraceTypeQuery1" true))
  (if _returnvalue
    (if (Class|KismetSystemLibrary|DoesClassImplementInterface (Utilities|GetClass (.hitactor _hitresult)) "/Game/actors/BI_CursorDetector.BI_CursorDetector_C")
      (if (not (== (.hitactor _hitresult) (Variables|Default|GetlastHitActor)))
        (if (Utilities|IsValid (Variables|Default|GetlastHitActor))
          (Class|BICursorDetector|UnHighlightActor(Message) (Variables|Default|GetlastHitActor)))
        (bind _asbi_cursor_detector (Utilities|Casting|CastToBI_CursorDetector (.hitactor _hitresult)))
        (Default|HighlightActor _asbi_cursor_detector)
        (Variables|Default|SetlastHitActor (.hitactor _hitresult)))
      (else
        (Utilities|IsValid (Variables|Default|GetlastHitActor) :!label _label
          (:Is%20Valid
            (Class|BICursorDetector|UnHighlightActor(Message) (Variables|Default|GetlastHitActor))
            (Variables|Default|SetlastHitActor 0)))))
    (else
      (goto _label))))

(fn PickCheck
  (bind _lasthitactor (Variables|Default|GetlastHitActor))
  (Utilities|IsValid _lasthitactor
    (:Is%20Valid
      (Utilities|IsValid (Variables|Default|GetLastSelectedActor)
        (:Is%20Valid
          (if (== (Variables|Default|GetLastSelectedActor) _lasthitactor)
            (Class|BICursorDetector|UnPick(Message) (Variables|Default|GetLastSelectedActor) :!label _label)
            (Variables|Default|SetLastSelectedActor 0)
            (else
              (Class|BICursorDetector|UnPick(Message) (Variables|Default|GetLastSelectedActor))
              (Variables|Default|SetLastSelectedActor 0)
              (bind _output_get (Variables|Default|SetLastSelectedActor _lasthitactor :!label _label_2))
              (Class|BICursorDetector|Pick(Message) _output_get))))
        (:Is%20Not%20Valid
          (goto _label_2))))
    (:Is%20Not%20Valid
      (CallFunction|HideCharacterInfo)
      (Utilities|IsValid (Variables|Default|GetLastSelectedActor)
        (:Is%20Valid
          (goto _label))))))

(fn InitUI
  (bind _self self)
  (bind _returnvalue (UserInterface|CreateWidget "/Game/UI/MainCharacterUI.MainCharacterUI_C" _self))
  (bind _output_get (Variables|Default|SetMainUI _returnvalue))
  (UserInterface|Viewport|AddtoViewport _output_get 0)
  (bind _returnvalue_2 (UserInterface|CreateWidget "/Game/UI/CharacterInfoUI.CharacterInfoUI_C" _self))
  (bind _output_get_2 (Variables|Default|SetCharacterInfoUI _returnvalue_2))
  (UserInterface|Viewport|AddtoViewport _output_get_2 0)
  (Widget|SetVisibility _output_get_2 "Hidden")
  (bind _returnvalue_3 (UserInterface|CreateWidget "/Game/UI/PauseMenuUI.PauseMenuUI_C" _self))
  (bind _output_get_3 (Variables|Default|SetPauseMenuUI _returnvalue_3))
  (UserInterface|Viewport|AddtoViewport _output_get_3 0)
  (Widget|SetVisibility _output_get_3 "Hidden"))

(fn HideCharacterInfo
  (Widget|SetVisibility (Variables|Default|GetCharacterInfoUI) "Hidden"))

(fn ShowCharacterInfo
  (params (character :type ST%20Character%20Object%20Reference))
  (bind _characterinfoui (Variables|Default|GetCharacterInfoUI))
  (Utilities|IsValid _characterinfoui
    (:Is%20Valid
      (Default|LoadCharacter _characterinfoui character)
      (Widget|SetVisibility _characterinfoui "Visible"))
    (:Is%20Not%20Valid
      (Development|PrintString "Character Info UI Invalid!" true true "(R=1.000000,G=0.000000,B=0.064239,A=1.000000)"))))

(fn ShowMainCharacterInfo
  (bind _returnvalue (Class|CharacterSearcher|Get))
  (CallFunction|ShowCharacterInfo (Variables|/Script/Heros_Of_ST.CharacterSearcher|GetcurrentControlledCharacter _returnvalue)))

(fn PauseGame
  (Game|SetGamePaused true)
  (Widget|SetVisibility (Variables|Default|GetMainUI) "Hidden")
  (Widget|SetVisibility (Variables|Default|GetCharacterInfoUI) "Hidden")
  (Widget|SetVisibility (Variables|Default|GetPauseMenuUI) "Visible")
  (Variables|Default|SetIsPaused true))

(fn ResumeGame
  (Game|SetGamePaused false)
  (Widget|SetVisibility (Variables|Default|GetMainUI) "Visible")
  (Widget|SetVisibility (Variables|Default|GetCharacterInfoUI) "Hidden")
  (Widget|SetVisibility (Variables|Default|GetPauseMenuUI) "Hidden")
  (Variables|Default|SetIsPaused false))